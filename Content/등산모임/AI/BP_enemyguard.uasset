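; BP_enemyguard is an AI guard enemy that patrols and chases the horror player character.
; It walks between random tagged actors, repeating after each successful move.
; AIPerception updates on BP_HorrorCharacter raise its speed and start a chase; forgetting the character lowers speed and resumes patrol.
; A "stop" command freezes it through zero CustomTimeDilation and blocks new chases, while any other command releases it.
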(event OnTargetPerceptionUpdated(AIPerception)
  (params (Actor :type Actor%20Object%20Reference) (Stimulus :type AI%20Stimulus%20Structure))
  (if (not (Variables|Default|GetIsStopped))
    (bind _asbp_horror_character (Utilities|Casting|CastToBP_HorrorCharacter Actor))
    (Variables|/Script/Engine.CharacterMovementComponent|SetMaxWalkSpeed (Variables|Character|GetCharacterMovement) 3e+02)
    (AI|AIMoveTo self "0, 0, 0" _asbp_horror_character 5.0 false)))

(event OnTargetPerceptionForgotten(AIPerception)
  (params (Actor :type Actor%20Object%20Reference))
  (Utilities|Casting|CastToBP_HorrorCharacter Actor)
  (Variables|/Script/Engine.CharacterMovementComponent|SetMaxWalkSpeed (Variables|Character|GetCharacterMovement) 2.5e+02)
  (bind _outactors (Actor|GetAllActorsOfClasswithTag 0 (Variables|Default|GetTag) :!label _label))
  (AI|AIMoveTo self "0, 0, 0" (.OutItem (Utilities|Array|Random _outactors)) 5.0 false
    (:OnSuccess
      (Utilities|FlowControl|Delay 0.2)
      (goto _label))))

(event Custom|OnTargetPerceptionForgotten_이벤트
  (params (Actor :type Actor%20Object%20Reference)))

(event EventBeginPlay
  (EventDispatchers|AssignOnTargetPerceptionForgotten (Variables|Default|GetAIPerception) (delegate Custom|OnTargetPerceptionForgotten_이벤트))
  (bind _outactors (Actor|GetAllActorsOfClasswithTag 0 (Variables|Default|GetTag) :!label _label))
  (AI|AIMoveTo self "0, 0, 0" (.OutItem (Utilities|Array|Random _outactors)) 5.0 false
    (:OnSuccess
      (Utilities|FlowControl|Delay 0.2)
      (goto _label))))

(event EventExcuteCommand
  (params (Command :type String))
  (if (Utilities|Enum|Equal(Enum) Command "stop")
    (Variables|Default|SetCustomTimeDilation 0.0)
    (Variables|Default|SetIsStopped true)
    (else
      (Variables|Default|SetCustomTimeDilation 1.0)
      (Variables|Default|SetIsStopped false))))

(fn ConstructionScript)
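; BP_movement is an actor that moves back and forth along a straight line, reversing on a timer.
; Each tick it offsets itself along the normalized Direction vector at Speed scaled by delta time, without sweeping for collisions.
; A looping timer started on BeginPlay negates Direction every Timetochange seconds, so the travel distance follows from speed and interval rather than set endpoints.
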(event Custom|changedirection
  (Variables|Default|SetDirection (* (Variables|Default|GetDirection) -1)))

(event EventBeginPlay
  (Utilities|Time|SetTimerbyEvent (delegate Custom|changedirection) (Variables|Default|GetTimetochange) true))

(event Collision|EventActorBeginOverlap
  (params (OtherActor :type Actor%20Object%20Reference)))

(event EventTick
  (params (DeltaSeconds :type Float%20%28single-precision%29))
  (Transformation|AddActorWorldOffset (* (Math|Vector|Normalize (Variables|Default|GetDirection)) (* (Variables|Default|GetSpeed) (Utilities|Time|GetWorldDeltaSeconds)))))

(fn ConstructionScript)
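; BP_Commander is an in-game command console that sends typed "Target.Message" commands to actors through a text input widget.
; ToggleCommanderInput focuses the input box, while ExcuteCommand unwraps "command(...)" strings for ProcessCommand.
; ProcessCommand sends an empty message to all BPI_Command actors, then the message to those whose display name matches the target.
; It colours the widget green or red by result, echoes the input and restores game-only input.
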(event Custom|ToggleCommanderInput
  (bind _returnvalue (Class|InputDeviceLibrary|GetPlayerControllerfromInputDevice))
  (Input|SetInputModeGameandUI _returnvalue (Variables|/Game/등산모임/Commander/WBP_TextInput.WBP_TextInput_C|GetInputBox (Variables|Default|GetTextInputWidget)) "LockAlways" true false))

(event Custom|ProcessCommand
  (params (CommandText :type String))
  (bind (_lefts _rights _returnvalue) (Utilities|String|Split CommandText "."))
  (bind _textinputwidget (Variables|Default|GetTextInputWidget))
  (bind _textinputwidget_2 (Variables|Default|GetTextInputWidget))
  (bind _border_0 (Variables|/Game/등산모임/Commander/WBP_TextInput.WBP_TextInput_C|GetBorder_0 _textinputwidget))
  (bind _inputbox (Variables|/Game/등산모임/Commander/WBP_TextInput.WBP_TextInput_C|GetInputBox _textinputwidget_2))
  (bind _outactors (Actor|GetAllActorswithInterface "/Game/등산모임/Commander/BPI_Command.BPI_Command_C"))
  (for _array_element _outactors
    (Class|BPICommand|ExcuteCommand(Message) _array_element))
  (if _returnvalue
    (bind _array_element_2 (Utilities|Array|ForEachLoopwithBreak _outactors)
      (:LoopBody
        (if (Utilities|Enum|Equal(Enum) (Utilities|GetDisplayName _array_element_2) _lefts)
          (bind _issuccess (Class|BPICommand|ExcuteCommand(Message) _array_element_2 _rights))))
      (:Completed
        (if _issuccess
          (Class|Border|SetContentColorandOpacity _border_0 (Math|Color|MakeColor 0.0 1.0 0.0))
          (else
            (Class|Border|SetContentColorandOpacity _border_0 (Math|Color|MakeColor 1.0 0.0 0.0) :!label _label)))
        (bind _returnvalue_2 (Class|InputDeviceLibrary|GetPlayerControllerfromInputDevice))
        (Input|SetInputModeGameOnly _returnvalue_2 false)
        (Rendering|Components|TextRender|SetText (Variables|/Game/등산모임/Commander/WBP_TextInput.WBP_TextInput_C|GetDisplayBox _textinputwidget_2) (Utilities|Text|ToText(String) (Utilities|String|Append ">" (Utilities|String|ToString(Text) (Variables|/Script/UMG.EditableText|GetText _inputbox)))))
        (Rendering|Components|TextRender|SetText _inputbox "")))
    (else
      (goto _label))))

(event EventBeginPlay
  (bind _aswbp_text_input (Utilities|Casting|CastToWBP_TextInput (UserInterface|GetUserWidgetObject (Variables|Default|GetCommanderWidget))))
  (bind _output_get (Variables|Default|SetTextInputWidget _aswbp_text_input))
  (Variables|/Game/등산모임/Commander/WBP_TextInput.WBP_TextInput_C|SetParentCommander _output_get self))

(fn ConstructionScript)

(fn ExcuteCommand
  (params (Command :type String))
  (if (and (Utilities|String|StartsWith Command "command(") (Utilities|String|EndsWith Command ")"))
    (CallFunction|ProcessCommand (Utilities|String|RightChop (Utilities|String|LeftChop Command 1) 8))
    (return true)
    (else
      (return false))))
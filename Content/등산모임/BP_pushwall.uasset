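; BP_pushwall is an actor that pushes horror characters standing inside its trigger box in a fixed direction.
; Box overlap events add and remove each BP_HorrorCharacter in an OverlappingCharacters list.
; Every tick, it feeds movement input along the Arrow component's forward vector to each listed character, so the arrow sets the push direction.
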(event OnComponentBeginOverlap(Box)
  (params (OverlappedComponent :type Primitive%20Component%20Object%20Reference) (OtherActor :type Actor%20Object%20Reference) (OtherComp :type Primitive%20Component%20Object%20Reference) (OtherBodyIndex :type Integer) (bFromSweep :type Boolean) (SweepResult :type Hit%20Result%20Structure%20%28by%20ref%29))
  (bind _asbp_horror_character (Utilities|Casting|CastToBP_HorrorCharacter OtherActor))
  (Utilities|Array|AddUnique (Variables|Default|GetOverlappingCharacters) _asbp_horror_character))

(event OnComponentEndOverlap(Box)
  (params (OverlappedComponent :type Primitive%20Component%20Object%20Reference) (OtherActor :type Actor%20Object%20Reference) (OtherComp :type Primitive%20Component%20Object%20Reference) (OtherBodyIndex :type Integer))
  (bind _asbp_horror_character (Utilities|Casting|CastToBP_HorrorCharacter OtherActor))
  (Utilities|Array|RemoveItem (Variables|Default|GetOverlappingCharacters) _asbp_horror_character))

(event EventTick
  (params (DeltaSeconds :type Float%20%28single-precision%29))
  (for _array_element (Variables|Default|GetOverlappingCharacters)
    (Pawn|Input|AddMovementInput _array_element (Math|Vector|GetForwardVector (Variables|Default|GetArrow)) 5.0 false)))

(fn ConstructionScript)